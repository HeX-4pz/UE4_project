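; Player Blueprint for the Wolf and Eggs game that turns keyboard input into wolf movement.
; On BeginPlay it spawns the BPWolf actor at a fixed location, turns off replication on its Sprite, and adds the HUD widget to the viewport.
; The A, Z, X and D keys call the spawned wolf's move functions for the top-left, bottom-left, bottom-right and top-right positions.
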(event `self.ReceiveBeginPlay`
  (set `self.wasCalled` true)
  (bind _returnvalue (`|SpawnActorFromClass` "/Game/WolfAndEggs/Blueprints/BPWolf.BPWolf_C" (`KismetMathLibrary.MakeTransform` (0.0 15.0 0.0)) "DontSpawnIfColliding" "OverrideRootScale" null null))
  (set `self.AWolf` _returnvalue)
  (`ActorComponent.SetIsReplicated` (`self.Sprite`) false)
  (bind _returnvalue_2 (`|CreateWidget` "/Game/WolfAndEggs/Blueprints/HUD.HUD_C"))
  (bind _output_get (set `self.MyHud` _returnvalue_2))
  (`UserWidget.AddToViewport` _output_get 0))

(event `Key|A`
  (params (Key :type "Key Structure"))
  (:`Pressed`
    (`/Game/WolfAndEggs/Blueprints/BPWolf.moveTopLeft` (`self.AWolf`))))

(event `Key|Z`
  (params (Key :type "Key Structure"))
  (:`Pressed`
    (`/Game/WolfAndEggs/Blueprints/BPWolf.moveBottomLeft` (`self.AWolf`))))

(event `Key|X`
  (params (Key :type "Key Structure"))
  (:`Pressed`
    (`/Game/WolfAndEggs/Blueprints/BPWolf.moveBottomRight` (`self.AWolf`))))

(event `Key|D`
  (params (Key :type "Key Structure"))
  (:`Pressed`
    (`/Game/WolfAndEggs/Blueprints/BPWolf.moveTopRight` (`self.AWolf`))))

(fn `UserConstructionScript`)