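; Game mode for the Wolf and Eggs game, running egg spawning, score, fails and game over.
; A self-rescheduling timer spawns eggs on random roll paths; RandomInteger(3) never selects the fourth, bottom-right path.
; Every fifth point briefly shows a rabbit and shortens roll and spawn times by 20%.
; Fails reveal HUD markers; the third stops spawning, saves score to the game instance and notifies the Player.
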(event `self.ReceiveBeginPlay`
  (`KismetSystemLibrary.K2_SetTimer` null "SpawnEgg" (`self.NextEggTime`))
  (set `self.RollTime` 1.0)
  (set `self.Fail` 0)
  (`self.AddScore`))

(fn `AddFail`
  (locals (char :type "/Game/WolfAndEggs/Blueprints/Player Object Reference"))
  (bind _asplayer (cast `/Game/WolfAndEggs/Blueprints/Player` (`GameplayStatics.GetPlayerCharacter` 0)))
  (bind _output_get (set `local.char` _asplayer))
  (switch `int` (`self.Fail`)
    (:`0`
      (bind _myhud (`/Game/WolfAndEggs/Blueprints/Player.MyHud` _output_get))
      (`Widget.SetVisibility` (`/Game/WolfAndEggs/Blueprints/HUD.fail_1` _myhud) "Visible"))
    (:`1`
      (`Widget.SetVisibility` (`/Game/WolfAndEggs/Blueprints/HUD.fail_2` _myhud) "Visible"))
    (:`2`
      (`Widget.SetVisibility` (`/Game/WolfAndEggs/Blueprints/HUD.fail_3` _myhud) "Visible")))
  (bind _result (`/Engine/EditorBlueprintResources/StandardMacros.IncrementInt` (`self.Fail`))
    (:`  `
      (if (== _result 3)
        (`self.GameOver`)))))

(fn `AddScore`
  (bind _result (`/Engine/EditorBlueprintResources/StandardMacros.IncrementInt` (`self.Score`))
    (:`  `
      (if (and (> (`self.Score`) 0) (== (mod (`self.Score`) 5) 0))
        (`self.ShowRabbit`))
      (set `self.FormatedScore` (`|FormatText` (`KismetTextLibrary.Conv_IntToText` _result false false 4))))))

(fn `GameOver`
  (set `self.IsGameOver` true)
  (bind _ascustom_game_instance (cast `/Game/WolfAndEggs/Blueprints/CustomGameInstance` (`GameplayStatics.GetGameInstance`)))
  (`/Game/WolfAndEggs/Blueprints/CustomGameInstance.SetScore` _ascustom_game_instance (`self.Score`))
  (bind _asplayer (cast `/Game/WolfAndEggs/Blueprints/Player` (`GameplayStatics.GetPlayerCharacter` 0)))
  (`/Game/WolfAndEggs/Blueprints/Player.GameOver` _asplayer))

(fn `HideRabit`
  (`self.K2_DestroyActor` (`self.Rabit`)))

(fn `ShowRabbit`
  (bind _returnvalue (`|SpawnActorFromClass` "/Game/WolfAndEggs/Blueprints/BPRabit.BPRabit_C" (`KismetMathLibrary.MakeTransform` (`KismetMathLibrary.MakeVector` -220.0 15.0 170.0)) "Undefined" "OverrideRootScale" null null))
  (set `self.Rabit` _returnvalue)
  (`KismetSystemLibrary.K2_SetTimer` null "HideRabit" 3.0)
  (set `self.RollTime` (* (`self.RollTime`) 0.8))
  (set `self.NextEggTime` (* (`self.NextEggTime`) 0.8)))

(fn `SpawnEgg`
  (if (not (`self.IsGameOver`))
    (switch `int` (`KismetMathLibrary.RandomInteger` 3)
      (:`0`
        (set `self.GeneratedEggType` "NewEnumerator0")
        (set `self.EggSpawnPlaces` (`self.TopLeftRollPath`)))
      (:`1`
        (set `self.GeneratedEggType` "NewEnumerator1")
        (set `self.EggSpawnPlaces` (`self.TopRightRollPath`)))
      (:`2`
        (set `self.GeneratedEggType` "NewEnumerator2")
        (set `self.EggSpawnPlaces` (`self.BottomLeftRollPath`)))
      (:`3`
        (set `self.GeneratedEggType` "NewEnumerator3")
        (set `self.EggSpawnPlaces` (`self.BottomRightRollPath`))))
    (bind _returnvalue (`|SpawnActorFromClass` "/Game/WolfAndEggs/Blueprints/BPEgg.BPEgg_C" (`KismetMathLibrary.MakeTransform` (`|GetArrayItem` (`self.EggSpawnPlaces`))) "AlwaysSpawn" "OverrideRootScale" null null))
    (set `/Game/WolfAndEggs/Blueprints/BPEgg.RollPath` (`self.EggSpawnPlaces`) _returnvalue)
    (set `/Game/WolfAndEggs/Blueprints/BPEgg.EggType` (`self.GeneratedEggType`) _returnvalue)
    (`KismetSystemLibrary.K2_SetTimer` null "SpawnEgg" (`self.NextEggTime`))))

(fn `UserConstructionScript`)