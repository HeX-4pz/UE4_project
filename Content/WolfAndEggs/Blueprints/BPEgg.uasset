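; Egg actor for the Wolf and Eggs game that rolls down one of four chutes toward the wolf.
; A repeating timer, paced by the game mode, steps it along RollPath, rotating it by side, and destroys it on game over.
; At the path's end it scores if the wolf's state matches its EggType.
; Otherwise it shows a broken sprite, records a fail and later spawns a chick moving off sideways.
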(event `self.ReceiveBeginPlay`
  (bind _aswolf_game_mode (cast `/Game/WolfAndEggs/Blueprints/WolfGameMode` (`GameplayStatics.GetGameMode`)))
  (set `self.RollTime` (`/Game/WolfAndEggs/Blueprints/WolfGameMode.RollTime` _aswolf_game_mode))
  (`KismetSystemLibrary.K2_SetTimer` null "Roll" (`self.RollTime`)))

(fn `BreakEgg`
  (`PaperSpriteComponent.SetSprite` (`self.PaperSprite`) "/Game/sprites/egg_broken_Sprite.egg_broken_Sprite")
  (`self.K2_SetActorTransform` (`KismetMathLibrary.MakeTransform` (`|GetArrayItem` (`self.RollPath`) 5)))
  (`KismetSystemLibrary.K2_SetTimer` null "SpawnChick" 2.0)
  (bind _aswolf_game_mode (cast `/Game/WolfAndEggs/Blueprints/WolfGameMode` (`GameplayStatics.GetGameMode`)))
  (`/Game/WolfAndEggs/Blueprints/WolfGameMode.AddFail` _aswolf_game_mode))

(fn `CollectEgg`
  (bind _aswolf_game_mode (cast `/Game/WolfAndEggs/Blueprints/WolfGameMode` (`GameplayStatics.GetGameMode`)))
  (`/Game/WolfAndEggs/Blueprints/WolfGameMode.AddScore` _aswolf_game_mode)
  (`self.K2_DestroyActor`))

(fn `Get CounterclockwiseRoll`
  (returns (ReturnValue :type "Transform Structure"))
  (return (`KismetMathLibrary.MakeTransform` (`|GetArrayItem` (`self.RollPath`) (`self.CurrentIteration`)) (`KismetMathLibrary.MakeRotator` (.roll (`self.K2_GetActorRotation`)) (+ (.pitch (`self.K2_GetActorRotation`)) 45.0) (.yaw (`self.K2_GetActorRotation`))))))

(fn `GetClockwiseRoll`
  (returns (ReturnValue :type "Transform Structure"))
  (return (`KismetMathLibrary.MakeTransform` (`|GetArrayItem` (`self.RollPath`) (`self.CurrentIteration`)) (`KismetMathLibrary.MakeRotator` (.roll (`self.K2_GetActorRotation`)) (+ (.pitch (`self.K2_GetActorRotation`)) -45.0) (.yaw (`self.K2_GetActorRotation`))))))

(fn `Roll`
  (bind _aswolf_game_mode (cast `/Game/WolfAndEggs/Blueprints/WolfGameMode` (`GameplayStatics.GetGameMode`)))
  (if (`/Game/WolfAndEggs/Blueprints/WolfGameMode.IsGameOver` _aswolf_game_mode)
    (`self.K2_DestroyActor`)
    (elif (< (`self.CurrentIteration`) 4)
      (set `self.CurrentIteration` (+ (`self.CurrentIteration`) 1))
      (switch `/Game/WolfAndEggs/Blueprints/BEWolfStates` (`self.EggType`)
        (:`NewEnumerator0`
          (bind _returnvalue (`self.GetClockwiseRoll` :!label _label))
          (`self.K2_SetActorTransform` _returnvalue))
        (:`NewEnumerator1`
          (bind _returnvalue_2 (`self.Get CounterclockwiseRoll` :!label _label_2))
          (`self.K2_SetActorTransform` _returnvalue_2))
        (:`NewEnumerator2`
          (goto _label))
        (:`NewEnumerator3`
          (goto _label_2)))
      (`KismetSystemLibrary.K2_SetTimer` null "Roll" (`self.RollTime`))
      (else
        (bind _asplayer (cast `/Game/WolfAndEggs/Blueprints/Player` (`GameplayStatics.GetPlayerCharacter` 0)))
        (if (`|EnumEquality` (`/Game/WolfAndEggs/Blueprints/BPWolf.mState` (`/Game/WolfAndEggs/Blueprints/Player.AWolf` _asplayer)) (`self.EggType`))
          (`self.CollectEgg`)
          (else
            (`self.BreakEgg`)))))))

(fn `SpawnChick`
  (`self.K2_DestroyActor`)
  (bind _returnvalue (`|SpawnActorFromClass` "/Game/WolfAndEggs/Blueprints/BPChick.BPChick_C" (`KismetMathLibrary.MakeTransform` (`|GetArrayItem` (`self.RollPath`) 5)) "Undefined" "OverrideRootScale" null null))
  (switch `/Game/WolfAndEggs/Blueprints/BEWolfStates` (`self.EggType`)
    (:`NewEnumerator0`
      (bind _projectilemovement (`/Game/WolfAndEggs/Blueprints/BPChick.ProjectileMovement` _returnvalue))
      (`ProjectileMovementComponent.SetVelocityInLocalSpace` _projectilemovement (-70.0 0.0 0.0) :!label _label))
    (:`NewEnumerator1`
      (`ProjectileMovementComponent.SetVelocityInLocalSpace` _projectilemovement (70.0 0.0 0.0) :!label _label_2))
    (:`NewEnumerator2`
      (goto _label))
    (:`NewEnumerator3`
      (goto _label_2))))

(fn `UserConstructionScript`)