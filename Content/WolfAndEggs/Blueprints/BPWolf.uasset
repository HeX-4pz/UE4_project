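; BPWolf is the player-style wolf actor in the WolfAndEggs game, shown as a Paper2D sprite in one of four catching poses.
; Four move events set the MState enum and call UpdatePosition, and BeginPlay starts it at bottom right.
; UpdatePosition teleports the actor to a fixed left or right spot and swaps the sprite, so top and bottom differ only by sprite.
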(event `self.ReceiveBeginPlay`
  (set `self.mState` "NewEnumerator3")
  (`self.UpdatePosition`))

(event `moveTopLeft`
  (set `self.mState` "NewEnumerator0")
  (`self.UpdatePosition` :!label _label))

(event `moveBottomLeft`
  (set `self.mState` "NewEnumerator2")
  (goto _label))

(event `moveBottomRight`
  (set `self.mState` "NewEnumerator3")
  (goto _label))

(event `moveTopRight`
  (set `self.mState` "NewEnumerator1")
  (goto _label))

(fn `UpdatePosition`
  (switch `/Game/WolfAndEggs/Blueprints/BEWolfStates` (`self.mState`)
    (:`NewEnumerator0`
      (`self.K2_SetActorLocation` (-80.0 15.0 -70.0) false true)
      (`PaperSpriteComponent.SetSprite` (`self.PaperSprite`) "/Game/sprites/wolf_top_left_Sprite.wolf_top_left_Sprite"))
    (:`NewEnumerator1`
      (`self.K2_SetActorLocation` (70.0 15.0 -70.0) false true)
      (`PaperSpriteComponent.SetSprite` (`self.PaperSprite`) "/Game/sprites/wolf_top_right_Sprite.wolf_top_right_Sprite"))
    (:`NewEnumerator2`
      (`self.K2_SetActorLocation` (-80.0 15.0 -70.0) false true)
      (`PaperSpriteComponent.SetSprite` (`self.PaperSprite`) "/Game/sprites/wolf_bottom_left_Sprite.wolf_bottom_left_Sprite"))
    (:`NewEnumerator3`
      (`self.K2_SetActorLocation` (70.0 15.0 -70.0) false true)
      (`PaperSpriteComponent.SetSprite` (`self.PaperSprite`) "/Game/sprites/wolf_bottom_right_Sprite.wolf_bottom_right_Sprite"))))

(fn `UserConstructionScript`)