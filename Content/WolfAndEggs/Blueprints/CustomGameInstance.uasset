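; Game instance for the Wolf and Eggs game that keeps the score leaderboard across sessions.
; On init it loads the MySave slot and copies its leaderboard into Scores, only printing a debug string if that fails.
; SetScore rebuilds the list by carrying the new score down through it, dropping the last displaced value so the length stays fixed, then saves through a newly created MySave object.
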(event `self.ReceiveInit`
  (bind _returnvalue (`GameplayStatics.LoadGameFromSlot` "1"))
  (bind _asmy_save (cast `/Game/WolfAndEggs/Blueprints/MySave` _returnvalue)
    (:`then`
      (set `self.Scores` (`/Game/WolfAndEggs/Blueprints/MySave.LeaderBoard` _asmy_save)))
    (:`CastFailed`
      (`KismetSystemLibrary.PrintString` "Hello"))))

(fn `SetScore`
  (params (NewScore :type Integer))
  (locals (tmpScore :type "Array of Integer") (candidate :type Integer))
  (bind _candidate (`local.candidate`))
  (set `local.candidate` NewScore)
  (for _array_element (`self.Scores`)
    (if (> _array_element _candidate)
      (`KismetArrayLibrary.Array_Add` (`local.tmpScore`) _array_element)
      (else
        (`KismetArrayLibrary.Array_Add` (`local.tmpScore`) _candidate)
        (set `local.candidate` _array_element))))
  (set `self.Scores` (`local.tmpScore`))
  (bind _returnvalue (`GameplayStatics.CreateSaveGameObject` "/Game/WolfAndEggs/Blueprints/MySave.MySave_C"))
  (`/Game/WolfAndEggs/Blueprints/MySave.Save` _returnvalue (`self.Scores`)))